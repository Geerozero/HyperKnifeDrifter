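; Spawn point actor that spawns an enemy of a selected class at its own location.
; The construction script maps the ClassToSpawn enum to one of three entries in EnemyClassCollection and stores it as EnemyClassToSpawn.
; The Spawn function creates that class at the root component's world location.
; As a test hook, BeginPlay enables player input so pressing U triggers Spawn.
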(event `self.ReceiveBeginPlay`
  ;[1 1 1] TEST: getting input
  (`self.EnableInput` (`GameplayStatics.GetPlayerController` 0)))

(event `Key|U`
  (params (Key :type "Key Structure"))
  ;[1 1 1] Test case
  (:`Pressed`
    (`self.Spawn`)))

(fn `Spawn`
  ;[1 1 1] Spawn class on location of this spawn point
  (`|SpawnActorFromClass` (`self.EnemyClassToSpawn`) (`KismetMathLibrary.MakeTransform` (`SceneComponent.K2_GetComponentLocation` (`self.DefaultSceneRoot`))) "Undefined" "OverrideRootScale" null null))

(fn `UserConstructionScript`
  (if (`|EnumEquality` (`self.ClassToSpawn`) "NewEnumerator0")
    (set `self.EnemyClassToSpawn` (`|GetArrayItem` (`self.EnemyClassCollection`)))
    (elif (`|EnumEquality` (`self.ClassToSpawn`) "NewEnumerator1")
      (set `self.EnemyClassToSpawn` (`|GetArrayItem` (`self.EnemyClassCollection`) 1))
      (elif (`|EnumEquality` (`self.ClassToSpawn`) "NewEnumerator2")
        (set `self.EnemyClassToSpawn` (`|GetArrayItem` (`self.EnemyClassCollection`) 2))))))