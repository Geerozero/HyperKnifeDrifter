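; Roller enemy that collapses and rolls at the player when in range, damaging Player-tagged actors it overlaps mid-roll.
; A self-calling detection event polls distance, then chains into a timed AI MoveTo roll, stop and recharge before detecting again.
; It takes damage only when not rolling, using EnemyStatComponent for health and death.
; Helper functions set collapse, roll and extend flags on RollerUnit_AnimBP; the FacePlayer timer is never wired to run.
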(event `Extend And Start Roll`
  ;[1 1 1] Start Roll
  (if (not (and (`self.isRecharging`) (`self.isRolling`)))
    (`self.AnimationIsExtendingToggle` false)
    (`self.AnimationIsCollapsingToggle` true)
    (`KismetSystemLibrary.RetriggerableDelay` 1.0)
    (`self.RollAtPlayer`)))

(event `Stop Roll And Reset`
  ;[1 1 1] Stops enemy and forces it to idle animation
  (if (not (`self.isRolling`))
    (`MovementComponent.StopMovementImmediately` (`self.CharacterMovement`))
    (`self.AnimationIsRollingToggle` false)
    (`self.AnimationIsExtendingToggle` true)
    (`self.AnimationIsCollapsingToggle` false)))

(event `DetectionRange`
  ;[1 1 1] Checks if player is within range of enemy
  (if (< (`self.GetDistanceTo` self (`GameplayStatics.GetPlayerCharacter` 0)) (`self.AttackRange`))
    ;[1 1 1] Collapses and rolls animation
    (`self.Extend And Start Roll`)
    (else
      ;[1 1 1] Stops rolls, and LOOPS
      (`self.Stop Roll And Reset`)
      (`KismetSystemLibrary.RetriggerableDelay` 0.5)
      (`self.DetectionRange`))))

(event `self.ReceiveBeginPlay`
  ;[1 1 1] Begins seeking player
  (`self.DetectionRange`))

(event `FacePlayer`
  (bind (_returnvalue_roll _returnvalue_pitch _returnvalue_yaw) (`KismetMathLibrary.BreakRotator` (`KismetMathLibrary.FindLookAtRotation` (`self.K2_GetActorLocation`) (`self.K2_GetActorLocation` (`GameplayStatics.GetPlayerCharacter` 0)))))
  ;[1 1 1] Rotates to player direction
  (if (`self.IsFacing`)
    (`self.K2_SetActorRotation` (`KismetMathLibrary.RInterpTo` (`self.K2_GetActorRotation`) (`KismetMathLibrary.MakeRotator` 0.0 0.0 _returnvalue_yaw) (`GameplayStatics.GetWorldDeltaSeconds`) 1.0))))

(event `RollAtPlayer`
  (bind _returnvalue (`GameplayStatics.GetPlayerCharacter` 0))
  ;[1 1 1] Roll at player
  (if (not (`self.isRolling`))
    (`self.AnimationIsRollingToggle` true)
    (set `self.isRolling` true)
    (`/Engine/EditorBlueprintResources/StandardMacros.IsValid` _returnvalue
      (:`Is Valid`
        (`|AIMoveTo` self (`self.K2_GetActorLocation` _returnvalue) _returnvalue 50.0
          (:`then`
            ;[1 1 1] Hunt roll for this amount of time
            (`KismetSystemLibrary.RetriggerableDelay` (`self.RollTime`))
            ;[1 1 1] Stop roll
            (set `self.isRolling` false)
            (set `self.isRecharging` true)
            (`self.Stop Roll And Reset`)
            ;[1 1 1] Time to recharge
            (`KismetSystemLibrary.RetriggerableDelay` (`self.RechargeTime`))
            (set `self.isRecharging` false)
            ;[1 1 1] Call animation and loop
            (`self.DetectionRange`))
          (:`OnSuccess`
            ;[1 1 1] On success stop animation early
            (`self.AnimationIsRollingToggle` false)
            (`self.AnimationIsExtendingToggle` true)))))))

(event `self.DamageCapsule.OnComponentBeginOverlap`
  (params (OverlappedComponent :type "PrimitiveComponent Object Reference") (OtherActor :type "Actor Object Reference") (OtherComp :type "PrimitiveComponent Object Reference") (OtherBodyIndex :type Integer) (bFromSweep :type Boolean) (SweepResult :type "HitResult Structure (by ref)"))
  ;[1 1 1] Only does damage while rolling
  (if (`self.isRolling`)
    (if (`self.ActorHasTag` OtherActor "Player")
      (`GameplayStatics.ApplyDamage` OtherActor (`/Game/Blueprints/EnemyStatComponent.AttackPower` (`self.EnemyStatComponent`)) null self))))

(event `self.ReceiveAnyDamage`
  (params (Damage :type "Float (single-precision)") (DamageType :type "DamageType Object Reference") (InstigatedBy :type "Controller Object Reference") (DamageCauser :type "Actor Object Reference"))
  (bind _enemystatcomponent (`self.EnemyStatComponent`))
  ;[1 1 1] General damage function
  (if (not (`self.isRolling`))
    (set `/Game/Blueprints/EnemyStatComponent.CurrentHealth` (- (`/Game/Blueprints/EnemyStatComponent.CurrentHealth` _enemystatcomponent) Damage) _enemystatcomponent)
    (`/Game/Blueprints/EnemyStatComponent.CheckStatus` _enemystatcomponent)
    (if (`/Game/Blueprints/EnemyStatComponent.IsDead?` _enemystatcomponent)
      (`self.K2_DestroyActor`))))

(fn `AnimationIsCollapsingToggle`
  (params (ToggleState :type Boolean))
  ;[1 1 1] Setting collapse animation
  (bind _asroller_unit_anim_bp (cast `/Game/Animation/RollerUnit_AnimBP` (`SkeletalMeshComponent.GetAnimInstance` (`self.Mesh`))))
  (set `/Game/Animation/RollerUnit_AnimBP.isCollapsing` ToggleState _asroller_unit_anim_bp))

(fn `AnimationIsExtendingToggle`
  (params (ToggleState :type Boolean))
  ;[1 1 1] Setting collapse animation
  (bind _asroller_unit_anim_bp (cast `/Game/Animation/RollerUnit_AnimBP` (`SkeletalMeshComponent.GetAnimInstance` (`self.Mesh`))))
  (set `/Game/Animation/RollerUnit_AnimBP.isExtending` ToggleState _asroller_unit_anim_bp))

(fn `AnimationIsRollingToggle`
  (params (ToggleState :type Boolean))
  ;[1 1 1] Setting collapse animation
  (bind _asroller_unit_anim_bp (cast `/Game/Animation/RollerUnit_AnimBP` (`SkeletalMeshComponent.GetAnimInstance` (`self.Mesh`))))
  (set `/Game/Animation/RollerUnit_AnimBP.isRolling` ToggleState _asroller_unit_anim_bp))

(fn `UserConstructionScript`
  (set `CharacterMovementComponent.MaxWalkSpeed` (`self.RollingSpeed`) (`self.CharacterMovement`)))