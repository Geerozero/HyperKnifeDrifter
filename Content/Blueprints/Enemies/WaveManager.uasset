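; Wave manager for a room encounter that locks the doors and spawns enemy waves until the room is cleared.
; The first overlap of the entry collision closes its assigned doors and spawns enemies at assigned spawn points whose wave number matches the current wave.
; Each spawned enemy receives a manager reference, and defeat notifications are counted against the spawn total to start the next wave or reopen the doors after the last.
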(event `self.ReceiveBeginPlay`
  ;[1 1 1] TEST: getting input
)

(event `self.EntryCollision.OnComponentBeginOverlap`
  (params (OverlappedComponent :type "PrimitiveComponent Object Reference") (OtherActor :type "Actor Object Reference") (OtherComp :type "PrimitiveComponent Object Reference") (OtherBodyIndex :type Integer) (bFromSweep :type Boolean) (SweepResult :type "HitResult Structure (by ref)"))
  ;[1 1 1] Only should activate once
  (if (not (`self.Wave Manager Activated?`))
    (`KismetSystemLibrary.PrintString` (`KismetSystemLibrary.GetDisplayName` OtherActor))
    ;[1 1 1] Door active only when player crposses activation point
    (if true
      ;[1 1 1] Open all doors, set this manager activated
      (set `self.Wave Manager Activated?` true)
      (`self.Close All Doors`)
      (`self.Start Wave Spawn`))))

(event `Next Wave`
  ;[1 0.18 0.1003] SPAWN
  ;;[1 1 1] Only called after enemies are defeated in previous wave
  (`KismetSystemLibrary.PrintText` (`|FormatText` "Spawn Wave {X}" (`self.WaveToSpawn`)))
  (`self.Spawn Wave` :!label _label))

(event `Key|U`
  (params (Key :type "Key Structure")))

(event `Start Wave Spawn`
  ;[1 0.18 0.1003] SPAWN
  ;;[1 1 1] START Spawning Waves
  (`KismetSystemLibrary.PrintString` "START Spawning Waves")
  (goto _label))

(event `/Game/Blueprints/Enemies/EnemyToManagerInterface.Notify Enemy Defeated`
  ;[1 1 1] Keep count of enemies defeated
  (bind _result (`/Engine/EditorBlueprintResources/StandardMacros.IncrementInt` (`self.Enemies Defeated`))
    (:`  `
      (`KismetSystemLibrary.PrintString` (`KismetTextLibrary.Conv_TextToString` (`|FormatText` "{X} enemies were defeated" _result)))
      (`self.Check If All Enemies Defeated`))))

(fn `Check If All Enemies Defeated`
  ;[1 1 1] Checks if number of enemies defeated == enemies spawned for wave
  (if (== (`self.Enemies Defeated`) (`self.Number Of Enemies Spawned`))
    ;[1 1 1] Reset variables
    (set `self.Enemies Defeated` 0)
    (set `self.Number Of Enemies Spawned` 0)
    ;[1 1 1] Check if this was the final wave
    (if (== (`self.WaveToSpawn`) (`self.NumberOfWavesSpawningInRoom`))
      ;[0.06004 1 0] OPENED DOORS
      (`KismetSystemLibrary.PrintString` "ROOM COMPLETE" true true (struct :`R` 0.039234 :`G` 1.0 :`A` 1.0))
      (`self.Open All Doors`)
      (else
        ;[1 1 1] Increment wave
        (set `self.WaveToSpawn` (+ (`self.WaveToSpawn`) 1))
        ;[1 1 1] Spawn next wave if all enemies are killed and more waves are available
        (`self.Next Wave`)))))

(fn `Close All Doors`
  ;[1 1 1] Close all doors
  (for _array_element (`self.Doors This Manager Opens/Closes`)
    (`/Game/Blueprints/Environment/PlaceholderDoor.CloseDoor` _array_element))
  (`KismetSystemLibrary.PrintString` "DOORS ALL OPEN"))

(fn `Open All Doors`
  ;[1 1 1] Open all doors
  (for _array_element (`self.Doors This Manager Opens/Closes`)
    (`/Game/Blueprints/Environment/PlaceholderDoor.OpenDoor` _array_element))
  (`KismetSystemLibrary.PrintString` "DOORS ALL OPEN"))

(fn `Spawn Wave`
  (for _array_element (`self.Spawn Points This Manager Uses`)
    ;[1 1 1] Check spawn points wave number, if it matches, spawn the enemy
    (if (== (`self.WaveToSpawn`) (`/Game/Blueprints/Enemies/SpawnPoint.SpawnPointWaveNumber` _array_element))
      ;;[1 1 1] Print what spawn point is spawning
      (`KismetSystemLibrary.PrintString` (`KismetSystemLibrary.GetDisplayName` _array_element) true true (struct :`R` 1.0 :`G` 0.460541 :`B` 0.550523 :`A` 1.0))
      (bind _spawned_enemy (`/Game/Blueprints/Enemies/SpawnPoint.Spawn` _array_element))
      (message `/Game/Blueprints/Enemies/ManagerToEnemyInterface.Wave Manager Reference Passing` _spawned_enemy self)
      ;[1 1 1] Note number of enemies spawned
      (`/Engine/EditorBlueprintResources/StandardMacros.IncrementInt` (`self.Number Of Enemies Spawned`))))
  ;[1 1 1] Just prints out how many enemies were spawned
  (`KismetSystemLibrary.PrintString` (`KismetTextLibrary.Conv_TextToString` (`|FormatText` "{X} enemies were spawned" (`self.Number Of Enemies Spawned`)))))

(fn `UserConstructionScript`)