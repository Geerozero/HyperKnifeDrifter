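; Stationary turret enemy that wakes when the player enters attack range, turns toward them and fires projectiles.
; Tick interpolates rotation toward the player and checks distance, toggling range state and starting a delayed, self-recalling Fire loop that stops out of range.
; Helper functions set AnimBP flags for wake, charge and shot.
; Damage reduces EnemyStatComponent health; on death the turret notifies its wave manager and destroys itself.
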(event `self.ReceiveBeginPlay`
  ;[1 1 1] Fire loop STARTED when in range
  ;;[1 1 1] Starts Fire Loop
)

(event `DetectionRange`
  ;[1 1 1] Checks if player is in distance of firing range
  (if (< (`self.GetDistanceTo` self (`GameplayStatics.GetPlayerCharacter` 0)) (`self.AttackRange`))
    ;[1 1 1] Only goes through if InRange? has not been set to this variable before
    (if (not (`self.InRange?`))
      ;[1 1 1] Set variable and animations
      (set `self.InRange?` true)
      (`self.AnimationIsAwakeToggle` true)
      ;[1 1 1] Delay before firing
      (`KismetSystemLibrary.Delay` 0.5)
      (`self.AnimationIsAttackStartToggle` true)
      (`KismetSystemLibrary.Delay` 1.0)
      ;[1 1 1] Begin fire loop
      (`self.Fire`))
    (elif (`self.InRange?`)
      (set `self.InRange?` false)
      (`self.AnimationIsAwakeToggle` false)
      ;[1 1 1] Set appropriate variables off
      (set `self.isNotFiring` true)
      (`self.AnimationAttackChargeDone` false)
      (`self.AnimationIsAttackStartToggle` false))))

(event `/Game/Blueprints/Enemies/ManagerToEnemyInterface.Wave Manager Reference Passing`
  (params (`Wave Manager Passing Message` :type "/Game/Blueprints/Enemies/WaveManager Object Reference"))
  ;[1 1 1] Wave manager being passed in
  (set `self.WaveManagerReference` `Wave Manager Passing Message`))

(event `self.ReceiveTick`
  (params (DeltaSeconds :type "Float (single-precision)"))
  (`self.TurretRotation`)
  (`self.DetectionRange`))

(event `TurretRotation`
  ;[1 1 1] Rotates to player when in range
  (if (`self.InRange?`)
    (`SceneComponent.K2_SetWorldRotation` (`self.CapsuleComponent`) (`KismetMathLibrary.RInterpTo` (`self.K2_GetActorRotation`) (`KismetMathLibrary.MakeRotator` 0.0 (.pitch (`KismetMathLibrary.FindLookAtRotation` (`self.K2_GetActorLocation`) (`self.K2_GetActorLocation` (`GameplayStatics.GetPlayerCharacter` 0)))) (.yaw (`KismetMathLibrary.FindLookAtRotation` (`self.K2_GetActorLocation`) (`self.K2_GetActorLocation` (`GameplayStatics.GetPlayerCharacter` 0))))) (`GameplayStatics.GetWorldDeltaSeconds`) (`self.RotationSpeed`)) false false)))

(event `self.ReceiveAnyDamage`
  (params (Damage :type "Float (single-precision)") (DamageType :type "DamageType Object Reference") (InstigatedBy :type "Controller Object Reference") (DamageCauser :type "Actor Object Reference"))
  (bind _enemystatcomponent (`self.EnemyStatComponent`))
  ;[1 1 1] Damage call
  (set `/Game/Blueprints/EnemyStatComponent.CurrentHealth` (- (`/Game/Blueprints/EnemyStatComponent.CurrentHealth` _enemystatcomponent) Damage) _enemystatcomponent)
  (`/Game/Blueprints/EnemyStatComponent.CheckStatus` _enemystatcomponent)
  (if (`/Game/Blueprints/EnemyStatComponent.IsDead?` _enemystatcomponent)
    (`self.Defeated Enemy`)
    (`self.K2_DestroyActor`)))

(event `Fire`
  ;[1 1 1] Firing call made constanly
  ;[1 1 1] Only want one shot going on per time
  (if (`self.isNotFiring`)
    ;[1 1 1] Checks if player in range
    (if (`self.InRange?`)
      (`KismetSystemLibrary.Delay` 1.0)
      ;[1 1 1] Set variables for currently firing/set animation to fire
      (set `self.isNotFiring` false)
      (`self.AnimationIsAttackStartToggle` false)
      (`self.AnimationAttackChargeDone` true)
      ;[1 1 1] Delay for timing out attack charge with spawning projectile
      (`KismetSystemLibrary.Delay` 0.2)
      ;[1 1 1] Spawns in front of the turret
      (`|SpawnActorFromClass` "/Game/Blueprints/Enemies/TurretProjectile.TurretProjectile_C" (`SceneComponent.K2_GetComponentToWorld` (`self.ShootPoint`)) "Undefined" "OverrideRootScale" self null)
      ;[1 1 1] Delay for loop put here to give time to animation
      (`KismetSystemLibrary.Delay` (`self.FireRate`))
      ;[1 1 1] Delay before calling again
      (`self.AnimationIsAttackStartToggle` true)
      (`self.AnimationAttackChargeDone` false)
      (set `self.isNotFiring` true)
      (`self.Fire`)
      (else
        ;[1 1 1] Break loop, stop animations
        (`self.AnimationAttackChargeDone` false)
        (`self.AnimationIsAttackStartToggle` false)))))

(fn `AnimationAttackChargeDone`
  (params (`Is Attack Charge Done` :type Boolean))
  (bind _asturret_unit_anim_bp (cast `/Game/Animation/TurretUnit_AnimBP` (`SkeletalMeshComponent.GetAnimInstance` (`self.Mesh`))))
  (set `/Game/Animation/TurretUnit_AnimBP.isAttackChargeDone` `Is Attack Charge Done` _asturret_unit_anim_bp))

(fn `AnimationIsAttackStartToggle`
  (params (`Attack Start State` :type Boolean))
  (bind _asturret_unit_anim_bp (cast `/Game/Animation/TurretUnit_AnimBP` (`SkeletalMeshComponent.GetAnimInstance` (`self.Mesh`))))
  (set `/Game/Animation/TurretUnit_AnimBP.isAttackStart` `Attack Start State` _asturret_unit_anim_bp))

(fn `AnimationIsAwakeToggle`
  (params (`isWakingUp?` :type Boolean))
  ;[1 1 1] Set to opposite of other for animation
  (bind _asturret_unit_anim_bp (cast `/Game/Animation/TurretUnit_AnimBP` (`SkeletalMeshComponent.GetAnimInstance` (`self.Mesh`))))
  (bind _output_get (set `/Game/Animation/TurretUnit_AnimBP.isWakingUp` `isWakingUp?` _asturret_unit_anim_bp))
  (set `/Game/Animation/TurretUnit_AnimBP.isSleeping` (not _output_get) _asturret_unit_anim_bp))

(fn `Defeated Enemy`
  ;[1 1 1] Notify manager about enemy defeate
  (message `/Game/Blueprints/Enemies/EnemyToManagerInterface.Notify Enemy Defeated` (`self.WaveManagerReference`)))

(fn `UserConstructionScript`)