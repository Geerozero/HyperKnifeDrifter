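; ScrapperUnit is a melee enemy that chases the player, performs charged attacks and is destroyed when its health runs out.
; A recursive, delay-driven SeekPlayer loop moves it by AIMoveTo and triggers Attack within range, while a looping timer smooths yaw toward the player, pausing for attacks.
; Attack stops movement, drives anim-blueprint charge flags, then sphere-traces forward with debug drawing, damaging a Player-tagged hit using EnemyStatComponent stats.
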(event `self.ReceiveBeginPlay`
  ;[1 1 1] Starts player seeking and begins timer of facing the player
  (`self.SeekPlayer`)
  (`KismetSystemLibrary.K2_SetTimerDelegate` (delegate `FacePlayer`) 0.001 true))

(event `FacePlayer`
  (bind (_returnvalue_roll _returnvalue_pitch _returnvalue_yaw) (`KismetMathLibrary.BreakRotator` (`KismetMathLibrary.FindLookAtRotation` (`self.K2_GetActorLocation`) (`self.K2_GetActorLocation` (`GameplayStatics.GetPlayerCharacter` 0)))))
  ;[1 1 1] Rotates enemy to face player
  (if (`self.IsFacing`)
    (`self.K2_SetActorRotation` (`KismetMathLibrary.RInterpTo` (`self.K2_GetActorRotation`) (`KismetMathLibrary.MakeRotator` 0.0 0.0 _returnvalue_yaw) (`GameplayStatics.GetWorldDeltaSeconds`) 1.0))))

(event `SeekPlayer`
  (bind _returnvalue (`GameplayStatics.GetPlayerCharacter` 0))
  ;[1 1 1] Seeking player checks if attacking
  (if (`self.IsAttacking`)
    ;[1 1 1] Is currently attacking so stop moving
    (`MovementComponent.StopMovementImmediately` (`self.CharacterMovement`))
    (else
      ;[1 1 1] Has enemy chase player and then delays
      (`/Engine/EditorBlueprintResources/StandardMacros.IsValid` _returnvalue
        (:`Is Valid`
          (`|AIMoveTo` self (`self.K2_GetActorLocation` _returnvalue) _returnvalue 75.0
            (:`then`
              _)
            (:`OnSuccess`
              _)
            (:`OnFail`
              _))
          (`KismetSystemLibrary.Delay` 0.2)
          ;[1 1 1] Checks if distance to attack is close enough
          (if (>= (`self.GetDistanceTo` (`GameplayStatics.GetPlayerCharacter` 0)) (`self.AttackRange`))
            ;[1 1 1] Not close enough, keep facing player
            (set `self.IsPlayerClose` false)
            (`self.FacePlayer`)
            (else
              ;[1 1 1] Close enough, stop facing temporarily and Attack
              (set `self.IsPlayerClose` true)
              (set `self.IsFacing` false)
              (`self.Attack`)
              (`KismetSystemLibrary.Delay` 2.0)
              ;[1 1 1] Have facing be valid again
              (set `self.IsFacing` true)))
          ;[1 1 1] Loops
          (`self.SeekPlayer`))))))

(event `Attack`
  (bind _returnvalue (`SceneComponent.K2_GetComponentLocation` (`self.AttackPoint`)))
  ;[1 1 1] Attack should: Stop, charge, then attack
  ;[1 1 1] Stop movement
  (if (`NavMovementComponent.IsMovingOnGround` (`self.CharacterMovement`))
    (set `self.IsAttacking` true)
    (`MovementComponent.StopMovementImmediately` (`self.CharacterMovement`))
    ;[1 1 1] Animation and attack timing corner
    ;;[1 1 1] Start attack charge
    (`self.SetAnimationIsAttacking` true)
    ;;[1 1 1] CHARGE delay
    (`KismetSystemLibrary.Delay` 0.5)
    ;;[1 1 1] End attack charge, finish attack anim
    (`self.SetAnimationIsChargeDone` true)
    (`self.SetAnimationIsAttacking` false)
    ;[1 1 1] Cast out a hurtbox in the shape of a pill
    (bind (_outhits _returnvalue_2) (`KismetSystemLibrary.SphereTraceMulti` :`Start` _returnvalue :`End` (+ _returnvalue (* (`self.GetActorForwardVector`) 100.0)) :`Radius` 50.0 :`TraceChannel` "TraceTypeQuery2" :`bTraceComplex` true :`DrawDebugType` "ForDuration" :`DrawTime` 0.5))
    ;[1 1 1] Only loops if something was hit
    (if _returnvalue_2
      ;[1 1 1] Check ALL objects hit and filter for the Player
      (for _array_element _outhits
        _)
      (bind (_bblockinghit _binitialoverlap _time _distance _location _impactpoint _normal _impactnormal _physmat _hitactor) (`GameplayStatics.BreakHitResult` _array_element))
      ;[1 1 1] If false: player not hit
      (if (`self.ActorHasTag` _hitactor "Player")
        ;[1 1 1] If not dead: Slap enemy Player with damage
        (if (not (`/Game/Blueprints/EnemyStatComponent.IsDead?` (`self.EnemyStatComponent`)))
          (`GameplayStatics.ApplyDamage` _hitactor (`/Game/Blueprints/EnemyStatComponent.AttackPower` (`self.EnemyStatComponent`)) null self)
          ;[1 1 1] Return to seeking player
          (set `self.IsAttacking` false :!label _label)
          (`KismetSystemLibrary.Delay` 0.01)
          (`self.SetAnimationIsChargeDone` false)
          (`KismetSystemLibrary.Delay` 0.5)
          (`self.SeekPlayer`))
        (else
          (goto _label)))
      (else
        (goto _label)))))

(event `self.ReceiveAnyDamage`
  (params (Damage :type "Float (single-precision)") (DamageType :type "DamageType Object Reference") (InstigatedBy :type "Controller Object Reference") (DamageCauser :type "Actor Object Reference"))
  (bind _enemystatcomponent (`self.EnemyStatComponent`))
  ;[1 1 1] General damage function
  (set `/Game/Blueprints/EnemyStatComponent.CurrentHealth` (- (`/Game/Blueprints/EnemyStatComponent.CurrentHealth` _enemystatcomponent) Damage) _enemystatcomponent)
  (`/Game/Blueprints/EnemyStatComponent.CheckStatus` _enemystatcomponent)
  (if (`/Game/Blueprints/EnemyStatComponent.IsDead?` _enemystatcomponent)
    (`self.K2_DestroyActor`)))

(fn `SetAnimationIsAttacking`
  (params (IsAttackingStart :type Boolean))
  ;[1 1 1] Sets animation to start the attack animation and hold on charge
  (bind _asscrapper_unit_anim_bp (cast `/Game/Animation/ScrapperUnit_AnimBP` (`SkeletalMeshComponent.GetAnimInstance` (`self.Mesh`))))
  (set `/Game/Animation/ScrapperUnit_AnimBP.isAttacking` IsAttackingStart _asscrapper_unit_anim_bp))

(fn `SetAnimationIsChargeDone`
  (params (IsChargeDone :type Boolean))
  ;[1 1 1] Sets Boolean of Attack Animation to leave the rumbling animation
  (bind _asscrapper_unit_anim_bp (cast `/Game/Animation/ScrapperUnit_AnimBP` (`SkeletalMeshComponent.GetAnimInstance` (`self.Mesh`))))
  (set `/Game/Animation/ScrapperUnit_AnimBP.isAttackChargeDone` IsChargeDone _asscrapper_unit_anim_bp))

(fn `UserConstructionScript`
  (`self.SetActorTickEnabled` true))