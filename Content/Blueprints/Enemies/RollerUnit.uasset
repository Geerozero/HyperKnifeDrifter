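; Roller enemy that chases the player and performs a telegraphed forward charge attack.
; A recursive SeekPlayer loop uses AIMoveTo, then attacks when within AttackRange, while a looping timer smoothly yaws it toward the player except during attacks.
; Attack halts on the ground, winds up, then launches via a velocity-change impulse before stopping and resuming the chase.
; DamageCapsule overlaps hurt tagged players mid-attack; EnemyStatComponent tracks incoming damage and destroys the actor on death.
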(event `self.ReceiveBeginPlay`
  (`self.SeekPlayer`)
  (`KismetSystemLibrary.K2_SetTimerDelegate` (delegate `FacePlayer`) 0.001 true))

(event `FacePlayer`
  (bind (_returnvalue_roll _returnvalue_pitch _returnvalue_yaw) (`KismetMathLibrary.BreakRotator` (`KismetMathLibrary.FindLookAtRotation` (`self.K2_GetActorLocation`) (`self.K2_GetActorLocation` (`GameplayStatics.GetPlayerCharacter` 0)))))
  (if (`self.IsFacing`)
    (`self.K2_SetActorRotation` (`KismetMathLibrary.RInterpTo` (`self.K2_GetActorRotation`) (`KismetMathLibrary.MakeRotator` 0.0 0.0 _returnvalue_yaw) (`GameplayStatics.GetWorldDeltaSeconds`) 1.0))))

(event `SeekPlayer`
  (bind _returnvalue (`GameplayStatics.GetPlayerCharacter` 0))
  (if (`self.IsAttacking`)
    (`MovementComponent.StopMovementImmediately` (`self.CharacterMovement`))
    (else
      (`/Engine/EditorBlueprintResources/StandardMacros.IsValid` _returnvalue
        (:`Is Valid`
          (`|AIMoveTo` self (`self.K2_GetActorLocation` _returnvalue) _returnvalue 300.0
            (:`OnSuccess`
              _)
            (:`OnFail`
              _))
          (`KismetSystemLibrary.Delay` 0.2)
          (if (>= (`self.GetDistanceTo` (`GameplayStatics.GetPlayerCharacter` 0)) (`self.AttackRange`))
            (set `self.IsPlayerClose` false)
            (`self.FacePlayer`)
            (else
              (set `self.IsPlayerClose` true)
              (set `self.IsFacing` false)
              (`self.Attack`)
              (`KismetSystemLibrary.Delay` 2.0)
              (set `self.IsFacing` true)))
          (`self.SeekPlayer`))))))

(event `Attack`
  (if (`NavMovementComponent.IsMovingOnGround` (`self.CharacterMovement`))
    (set `self.IsAttacking` true)
    (`MovementComponent.StopMovementImmediately` (`self.CharacterMovement`))
    (`KismetSystemLibrary.Delay` 2.0)
    (`KismetSystemLibrary.PrintString` "AttackMove")
    (`CharacterMovementComponent.AddImpulse` (`self.CharacterMovement`) (* (`self.GetActorForwardVector`) 6000.0) true)
    (`KismetSystemLibrary.Delay` 0.5)
    (`MovementComponent.StopMovementImmediately` (`self.CharacterMovement`))
    (set `self.IsAttacking` false)
    (`self.SeekPlayer`)))

(event `self.DamageCapsule.OnComponentBeginOverlap`
  (params (OverlappedComponent :type "PrimitiveComponent Object Reference") (OtherActor :type "Actor Object Reference") (OtherComp :type "PrimitiveComponent Object Reference") (OtherBodyIndex :type Integer) (bFromSweep :type Boolean) (SweepResult :type "HitResult Structure (by ref)"))
  (if (and (`self.ActorHasTag` OtherActor "Player") (`self.IsAttacking`))
    (`GameplayStatics.ApplyDamage` OtherActor (`/Game/Blueprints/EnemyStatComponent.AttackPower` (`self.EnemyStatComponent`)) null self)))

(event `self.ReceiveAnyDamage`
  (params (Damage :type "Float (single-precision)") (DamageType :type "DamageType Object Reference") (InstigatedBy :type "Controller Object Reference") (DamageCauser :type "Actor Object Reference"))
  (bind _enemystatcomponent (`self.EnemyStatComponent`))
  (set `/Game/Blueprints/EnemyStatComponent.CurrentHealth` (- (`/Game/Blueprints/EnemyStatComponent.CurrentHealth` _enemystatcomponent) Damage) _enemystatcomponent)
  (`/Game/Blueprints/EnemyStatComponent.CheckStatus` _enemystatcomponent)
  (if (`/Game/Blueprints/EnemyStatComponent.IsDead?` _enemystatcomponent)
    (`self.K2_DestroyActor`)))

(fn `UserConstructionScript`)