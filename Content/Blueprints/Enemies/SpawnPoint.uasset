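; Enemy spawn point actor that spawns a Scrapper, Turret or Roller at its own location.
; The construction script maps the ClassToSpawn enum to a class from EnemyClassCollection.
; Spawn prints the point's wave number, creates that class at the scene root's location and rotation, and returns the new actor.
; The event graph holds only inactive test nodes, so spawning relies on an external call to Spawn.
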(event `self.ReceiveBeginPlay`
  ;[1 1 1] TEST: getting input
)

(event `Key|U`
  (params (Key :type "Key Structure"))
  ;[1 1 1] Test case
)

(fn `Set Class To Spawn`
  ;[1 1 1] Scrapper
  (if (`|EnumEquality` (`self.ClassToSpawn`) "NewEnumerator0")
    (set `self.EnemyClassToSpawn` (`|GetArrayItem` (`self.EnemyClassCollection`)))
    (else
      ;[1 1 1] Turret
      (if (`|EnumEquality` (`self.ClassToSpawn`) "NewEnumerator1")
        (set `self.EnemyClassToSpawn` (`|GetArrayItem` (`self.EnemyClassCollection`) 1))
        (else
          ;[1 1 1] Roller
          (if (`|EnumEquality` (`self.ClassToSpawn`) "NewEnumerator2")
            (set `self.EnemyClassToSpawn` (`|GetArrayItem` (`self.EnemyClassCollection`) 2))))))))

(fn `Spawn`
  (returns (`Spawned Enemy` :type "Actor Object Reference"))
  (bind _sceneroot (`self.SceneRoot`))
  ;[1 1 1] Spawn class on location of this spawn point
  (`KismetSystemLibrary.PrintString` (`KismetTextLibrary.Conv_TextToString` (`|FormatText` "Printing for Wave {X}" (`self.SpawnPointWaveNumber`))))
  (bind _returnvalue (`|SpawnActorFromClass` (`self.EnemyClassToSpawn`) (`KismetMathLibrary.MakeTransform` (`SceneComponent.K2_GetComponentLocation` _sceneroot) (`SceneComponent.K2_GetComponentRotation` _sceneroot)) "Undefined" "OverrideRootScale" null null))
  (return _returnvalue))

(fn `UserConstructionScript`
  (`self.Set Class To Spawn`))