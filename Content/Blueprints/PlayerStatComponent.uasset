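; Player stat component for health, death state, heal charges and dash count.
; RepNotify functions cast the owner to TopDownCharacter and copy health, max health and dash count to its HUD status bar.
; UseHeal adds fixed health when charges remain and health is below max, otherwise sets it to max, never decrementing charges.
; CheckStatus flags death at zero health, but its over-max branch and UpdateDash are self-assignments that change no values.
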(fn `CheckStatus`
  (bind _currenthealth (`self.CurrentHealth`))
  (if (<= _currenthealth 0.0)
    (set `self.isDead?` true)
    (elif (> _currenthealth (`self.CurrentMaxHealth`))
      (set `self.CurrentMaxHealth` (`self.CurrentMaxHealth`)))))

(fn `OnRep_CurrentHealth`
  (bind _astop_down_character (cast `/Game/Blueprints/TopDownExample/TopDownCharacter` (`self.GetOwner`)))
  (set `/Game/Widgets/CharacterStatusBar.CurrentHP` (`self.CurrentHealth`) (`/Game/Widgets/PlayerHUD.CharacterStatusBar` (`/Game/Blueprints/TopDownExample/TopDownCharacter.HUD` _astop_down_character))))

(fn `OnRep_CurrentMaxHealth`
  (bind _astop_down_character (cast `/Game/Blueprints/TopDownExample/TopDownCharacter` (`self.GetOwner`)))
  (set `/Game/Widgets/CharacterStatusBar.MaxHP` (`self.CurrentMaxHealth`) (`/Game/Widgets/PlayerHUD.CharacterStatusBar` (`/Game/Blueprints/TopDownExample/TopDownCharacter.HUD` _astop_down_character))))

(fn `OnRep_CurrentNumDashes`
  (bind _astop_down_character (cast `/Game/Blueprints/TopDownExample/TopDownCharacter` (`self.GetOwner`)))
  (set `/Game/Widgets/CharacterStatusBar.CurrentNumDashes` (`self.CurrentNumDashes`) (`/Game/Widgets/PlayerHUD.CharacterStatusBar` (`/Game/Blueprints/TopDownExample/TopDownCharacter.HUD` _astop_down_character))))

(fn `UpdateDash`
  (set `self.CurrentNumDashes` (`self.CurrentNumDashes`)))

(fn `UseHeal`
  (bind _currenthealth (`self.CurrentHealth`))
  (bind _currentmaxhealth (`self.CurrentMaxHealth`))
  (if (and (> (`self.HealCharges`) 0) (< _currenthealth _currentmaxhealth))
    (set `self.CurrentHealth` (+ _currenthealth 20.0))
    (else
      (set `self.CurrentHealth` (+ _currenthealth (+ _currentmaxhealth (* _currenthealth -1.0)))))))