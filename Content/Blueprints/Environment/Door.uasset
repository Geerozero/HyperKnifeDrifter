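; Door actor that opens or closes according to its IsOpen flag, animating its skeletal mesh and toggling blocking collision.
; OpenDoor and CloseDoor set IsOpen on the NuDoor_AnimBP anim instance and switch DoorCollider between no collision and query-and-physics.
; Tick re-applies the current state every frame, and a DoorCheck event runs the same check.
; Nothing in this graph changes IsOpen itself.
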(event `self.ReceiveTick`
  (params (DeltaSeconds :type "Float (single-precision)"))
  (if (`self.isOpen?`)
    (`self.OpenDoor`)
    (else
      (`self.CloseDoor`))))

(event `DoorCheck`
  (if (`self.isOpen?`)
    (`self.OpenDoor`)
    (else
      (`self.CloseDoor`))))

(fn `CloseDoor`
  ;[1 1 1] Close door animation
  (bind _asnu_door_anim_bp (cast `/Game/Animation/NuDoor_AnimBP` (`SkeletalMeshComponent.GetAnimInstance` (`self.SkeletalMesh (KEEP IT OFFSET)`))))
  (set `/Game/Animation/NuDoor_AnimBP.isOpen` false _asnu_door_anim_bp)
  ;[1 1 1] Turns on collision of center door
  (`PrimitiveComponent.SetCollisionEnabled` (`self.DoorCollider`) "QueryAndPhysics"))

(fn `OpenDoor`
  ;[1 1 1] Open door animation
  (bind _asnu_door_anim_bp (cast `/Game/Animation/NuDoor_AnimBP` (`SkeletalMeshComponent.GetAnimInstance` (`self.SkeletalMesh (KEEP IT OFFSET)`))))
  (set `/Game/Animation/NuDoor_AnimBP.isOpen` true _asnu_door_anim_bp)
  ;[1 1 1] Turns off collision of door
  (`PrimitiveComponent.SetCollisionEnabled` (`self.DoorCollider`) "NoCollision"))

(fn `UserConstructionScript`)