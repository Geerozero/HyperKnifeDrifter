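; Placeholder door actor that blocks or clears a passage by toggling a single DoorBlocker component.
; OpenDoor hides the blocker and disables its collision, while CloseDoor shows it and restores query and physics collision, with no animation.
; On BeginPlay it sets its initial state from the StartClosed flag, opening unless that flag is set.
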(event `self.ReceiveBeginPlay`
  ;[1 1 1] Doors generally start open
  (if (`self.Start Closed?`)
    (`self.CloseDoor`)
    (else
      (`self.OpenDoor`))))

(fn `CloseDoor`
  (bind _doorblocker (`self.DoorBlocker`))
  ;[1 1 1] Close door
  (`SceneComponent.SetVisibility` _doorblocker true false)
  (`PrimitiveComponent.SetCollisionEnabled` _doorblocker "QueryAndPhysics"))

(fn `OpenDoor`
  (bind _doorblocker (`self.DoorBlocker`))
  ;[1 1 1] Close door
  (`SceneComponent.SetVisibility` _doorblocker false false)
  (`PrimitiveComponent.SetCollisionEnabled` _doorblocker "NoCollision"))

(fn `UserConstructionScript`)